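; A score-gated door actor that opens when something enters its trigger box.
; On begin play it caches the player's FirstPersonCharacter.
; On box overlap, it checks that character's CubeScore against a threshold of ten, without filtering the overlapping actor.
; If met, a timeline lerps the Cube mesh between start and end positions; otherwise it plays a 2D sound.
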(event OnComponentBeginOverlap(Box)
  (params (OverlappedComponent :type Primitive%20Component%20Object%20Reference) (OtherActor :type Actor%20Object%20Reference) (OtherComp :type Primitive%20Component%20Object%20Reference) (OtherBodyIndex :type Integer) (bFromSweep :type Boolean) (SweepResult :type Hit%20Result%20Structure%20%28by%20ref%29))
  (if (>= (Variables|/Game/FirstPersonBP/Blueprints/FirstPersonCharacter.FirstPersonCharacter_C|GetCubeScore (Variables|Default|GetMyCharacter)) 10)
    (bind _newtrack_0 (Timeline|Doorthingy Play)
      (:Update
        (Transformation|SetRelativeLocationAndRotation (Variables|Default|GetCube) (Math|Vector|Lerp(Vector) (Variables|Default|Getstart) (Variables|Default|GetEnd) _newtrack_0) "0, 0, 0" false false))
      (:Finished
        (Utilities|FlowControl|Delay 0.2)))
    (else
      (Audio|PlaySound2D 0 1.0 1.0 0.0 0 0))))

(event EventBeginPlay
  (bind _asfirst_person_character (Utilities|Casting|CastToFirstPersonCharacter (Game|Player|GetPlayerPawn 0)))
  (Variables|Default|SetMyCharacter _asfirst_person_character))

(event Collision|EventActorBeginOverlap
  (params (OtherActor :type Actor%20Object%20Reference)))

(event EventTick
  (params (DeltaSeconds :type Float%20%28single-precision%29)))

(fn ConstructionScript)